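; Player controller for BasketFall that handles pawn switching, ability input, level restart and the level-finish screen.
; Q swaps possession between the character and the Ball, leaving the character only when it has no ball, and possession updates the active camera state.
; Left Shift toggles character sprint through walk speed, while E calls empty ball-ability stubs.
; Holding R shows a progress widget and reloads the level, and CreateLevelFinishWidget switches input to UI-only.
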(event Input|EnhancedActionEvents|EnhancedInputActionIA_RestartLevel
  (params (ActionValue :type Boolean) (ElapsedSeconds :type Float%20%28double-precision%29) (TriggeredSeconds :type Float%20%28double-precision%29) (InputAction :type Input%20Action%20Object%20Reference :default "/Game/Core/Input/Actions/IA_RestartLevel.IA_RestartLevel"))
  (bind _returnvalue (Game|Player|IsInputKeyDown "R"))
  (:Triggered
    (if _returnvalue
      (bind _returnvalue_2 (Game|GetCurrentLevelName true))
      (Game|OpenLevel(byName) (Utilities|String|StringToName _returnvalue_2))))
  (:Started
    (if _returnvalue
      (bind _returnvalue_3 (UserInterface|CreateWidget "/Game/UI/WBP_RestartLevel.WBP_RestartLevel_C"))
      (bind _output_get (Variables|Default|SetRestartingLevelUI _returnvalue_3))
      (UserInterface|Viewport|AddtoViewport _output_get 0)))
  (:Ongoing
    (if _returnvalue
      (Default|SetPercent (Variables|/Game/UI/WBP_RestartLevel.WBP_RestartLevel_C|GetProgressBar (Variables|Default|GetRestartingLevelUI)) ElapsedSeconds)))
  (:Canceled
    (bind _restartinglevelui (Variables|Default|GetRestartingLevelUI :!label _label)
      (:then
        (Widget|RemovefromParent _restartinglevelui)
        (Variables|Default|SetRestartingLevelUI 0))
      (:else)))
  (:Completed
    (goto _label)))

(event EventPossess
  (params (PossessedPawn :type Pawn%20Object%20Reference))
  (bind _returnvalue (Utilities|GetClass PossessedPawn))
  (if (not (== _returnvalue "/Game/BasketFallBlueprints/Ball.Ball_C"))
    (if (not (== _returnvalue "/Game/Characters/BP_BasketFall_Character.BP_BasketFall_Character_C"))
      (Development|PrintString "Controller posessed unknown actor/pawn")
      (else
        (Variables|Default|SetActiveCamera "NewEnumerator0")
        (Variables|Default|GetPlayerRef
          (:then)
          (:else
            (bind _asbp_basket_fall_character (Utilities|Casting|CastToBP_BasketFall_Character PossessedPawn))
            (Variables|Default|SetPlayerRef _asbp_basket_fall_character)))))
    (else
      (Variables|Default|SetActiveCamera "NewEnumerator1"))))

(event Input|KeyboardEvents|Q
  (params (Key :type Key%20Structure :default "None"))
  (:Pressed
    (switch Utilities|FlowControl|Switch|SwitchonCameras (Variables|Default|GetActiveCamera)
      (:NewEnumerator0
        (bind _playerref (Variables|Default|GetPlayerRef)
          (:then
            (if (not (Variables|/Game/Characters/BP_BasketFall_Character.BP_BasketFall_Character_C|GetHasBall? _playerref))
              (bind _returnvalue (Actor|GetActorOfClass "/Game/BasketFallBlueprints/Ball.Ball_C"))
              (Utilities|IsValid _returnvalue
                (:Is%20Valid
                  (Pawn|Possess _returnvalue)))))
          (:else)))
      (:NewEnumerator1
        (bind _returnvalue_2 (Actor|GetActorOfClass "/Game/Characters/BP_BasketFall_Character.BP_BasketFall_Character_C"))
        (Utilities|IsValid _returnvalue_2
          (:Is%20Valid
            (Pawn|Possess _returnvalue_2)))))))

(event Input|KeyboardEvents|E
  (params (Key :type Key%20Structure :default "None"))
  (:Pressed
    (CallFunction|ActivateBallAbility))
  (:Released
    (CallFunction|DeactivateBallAbility)))

(event Input|KeyboardEvents|LeftShift
  (params (Key :type Key%20Structure :default "None"))
  (:Pressed
    (CallFunction|ActivatePlayerAbility))
  (:Released
    (CallFunction|DeactivatePlayerAbility)))

(fn ConstructionScript)

(fn CreateLevelFinishWidget
  (params (Reason :type String))
  (bind _returnvalue (UserInterface|CreateWidget "/Game/UI/WBP_LevelFinish.WBP_LevelFinish_C" 0 Reason))
  (UserInterface|Viewport|AddtoViewport _returnvalue 0)
  (Variables|Default|SetbShowMouseCursor true)
  (Input|SetInputModeUIOnly self _returnvalue "DoNotLock" false))

(fn SprintAbility
  (params (Active :type Boolean))
  (bind _playerref (Variables|Default|GetPlayerRef))
  (bind _charactermovement (Variables|/Script/Engine.Character|GetCharacterMovement _playerref))
  (if Active
    (Variables|/Script/Engine.CharacterMovementComponent|SetMaxWalkSpeed _charactermovement 1.2e+03)
    (else
      (Variables|/Script/Engine.CharacterMovementComponent|SetMaxWalkSpeed _charactermovement 8e+02))))

(fn ActivatePlayerAbility
  (CallFunction|SprintAbility true))

(fn ActivateBallAbility)

(fn DeactivatePlayerAbility
  (CallFunction|SprintAbility false))

(fn DeactivateBallAbility)