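; BasketFall game instance that tracks which abilities are unlocked and enabled, plus the current player and ball abilities.
; On Init it loads both ability maps from an existing save and rebuilds the current abilities from DT_Abilities.
; Enabling an ability looks up its type and disables the current Player or Ball one, while Modifiers take no slot.
; Lock, unlock and disable only update the maps; nothing here writes the save.
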(event EventInit
  (bind _returnvalue (SaveGame|DoesSaveGameExist))
  (if _returnvalue
    (bind _returnvalue_2 (SaveGame|LoadGamefromSlot))
    (bind _asbasket_fall_save_game (Utilities|Casting|CastToBasketFall_SaveGame _returnvalue_2))
    (CallFunction|LoadAbilityInformation _asbasket_fall_save_game)))

(event EventShutdown)

(fn IsAbilityUnlocked
  (params (Ability :type Name))
  (return (.Value (Utilities|Map|Find (Variables|Default|GetAbilityLockMap) Ability))))

(fn IsAbilityEnabled
  (params (Ability :type Name))
  (return (.Value (Utilities|Map|Find (Variables|Default|GetAbilityEnablementMap) Ability))))

(fn EnableAbility
  (params (Ability :type Name))
  (bind _returnvalue (Utilities|GetDataTableRow "/Game/Core/Data/DT_Abilities.DT_Abilities" Ability)
    (:then
      (if (not (== (Utilities|Struct|BreakS_Ability (Utilities|Select :Index (.Type (Utilities|Struct|BreakS_Ability _returnvalue)) :NewEnumerator0 (Variables|Default|GetCurrentPlayerAbility) :NewEnumerator1 (Variables|Default|GetCurrentBallAbility) :NewEnumerator2 "")) ""))
        (CallFunction|DisableAbility (Utilities|Struct|BreakS_Ability (Utilities|Select :Index (.Type (Utilities|Struct|BreakS_Ability _returnvalue)) :NewEnumerator0 (Variables|Default|GetCurrentPlayerAbility) :NewEnumerator1 (Variables|Default|GetCurrentBallAbility) :NewEnumerator2 ""))))
      (switch Utilities|FlowControl|Switch|SwitchonE_AbilityType (.Type (Utilities|Struct|BreakS_Ability _returnvalue))
        (:NewEnumerator0
          (Variables|Default|SetCurrentPlayerAbility _returnvalue))
        (:NewEnumerator1
          (Variables|Default|SetCurrentBallAbility _returnvalue))
        (:NewEnumerator2
          _))
      (Utilities|Map|Add (Variables|Default|GetAbilityEnablementMap) (.Id (Utilities|Struct|BreakS_Ability _returnvalue)) true))))

(fn DisableAbility
  (params (Ability :type Name))
  (Utilities|Map|Add (Variables|Default|GetAbilityEnablementMap) Ability false))

(fn UnlockAbility
  (params (Ability :type Name))
  (Utilities|Map|Add (Variables|Default|GetAbilityLockMap) Ability true))

(fn LockAbility
  (params (Ability :type Name))
  (Utilities|Map|Add (Variables|Default|GetAbilityLockMap) Ability false))

(fn LoadAbilityInformation
  (params (LoadedSave :type Basket%20Fall%20Save%20Game%20Object%20Reference))
  (Variables|Default|SetAbilityEnablementMap (Variables|/Game/Core/BasketFall_SaveGame.BasketFall_SaveGame_C|GetAbilityEnablementMap LoadedSave))
  (Variables|Default|SetAbilityLockMap (Variables|/Game/Core/BasketFall_SaveGame.BasketFall_SaveGame_C|GetAbilityLockMap LoadedSave))
  (bind _keys (Utilities|Map|Keys (Variables|Default|GetAbilityEnablementMap)))
  (for _array_element _keys
    (if (.Value (Utilities|Map|Find (Variables|Default|GetAbilityEnablementMap) _array_element))
      (bind _returnvalue (Utilities|GetDataTableRow "/Game/Core/Data/DT_Abilities.DT_Abilities" _array_element)
        (:then
          (switch Utilities|FlowControl|Switch|SwitchonE_AbilityType (.Type (Utilities|Struct|BreakS_Ability _returnvalue))
            (:NewEnumerator0
              (Variables|Default|SetCurrentPlayerAbility _returnvalue))
            (:NewEnumerator1
              (Variables|Default|SetCurrentBallAbility _returnvalue))))))))